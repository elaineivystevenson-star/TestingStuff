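; ANS_WeaponAttack is an anim notify state that marks the window in an animation during which a character's active weapon is in its attack state.
; On begin and end, it casts the mesh owner to BP_CharacterBase and sets WeaponState on CurrentActiveWeapon, switching to the second enum value for the window and back to the first afterward.
; Owners that are not BP_CharacterBase are left untouched.
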(fn ReceivedNotifyBegin
  (params (MeshComp :type Skeletal%20Mesh%20Component%20Object%20Reference) (Animation :type Anim%20Sequence%20Base%20Object%20Reference) (TotalDuration :type Float%20%28single-precision%29) (EventReference :type Anim%20Notify%20Event%20Reference%20Structure%20%28by%20ref%29))
  (bind _asbp_character_base (Utilities|Casting|CastToBP_CharacterBase (Components|GetOwner MeshComp)))
  (Variables|/Game/Blueprints/WeaponBlueprints/BP_WeaponBase.BP_WeaponBase_C|SetWeaponState (Variables|/Game/PlayerAssets/BP_CharacterBase.BP_CharacterBase_C|GetCurrentActiveWeapon _asbp_character_base) "NewEnumerator1")
  (return false))

(fn ReceivedNotifyEnd
  (params (MeshComp :type Skeletal%20Mesh%20Component%20Object%20Reference) (Animation :type Anim%20Sequence%20Base%20Object%20Reference) (EventReference :type Anim%20Notify%20Event%20Reference%20Structure%20%28by%20ref%29))
  (bind _asbp_character_base (Utilities|Casting|CastToBP_CharacterBase (Components|GetOwner MeshComp)))
  (Variables|/Game/Blueprints/WeaponBlueprints/BP_WeaponBase.BP_WeaponBase_C|SetWeaponState (Variables|/Game/PlayerAssets/BP_CharacterBase.BP_CharacterBase_C|GetCurrentActiveWeapon _asbp_character_base) "NewEnumerator0")
  (return true))